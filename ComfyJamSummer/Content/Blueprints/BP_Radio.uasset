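; BP_Radio is a radio that spawns a sound at its mesh location on BeginPlay, starting with the first track in MusicArray.
; When the audio component finishes, NextSong rotates that track to the end of the array and sets the new first entry as the sound, treating the array as a looping playlist.
; A Skip event triggers the same rotation for manual skips and prints a message.
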(event Custom|RadioStart
  (bind _returnvalue (Audio|SpawnSoundatLocation (Utilities|Array|Get(acopy) (Variables|Default|GetMusicArray)) (Transformation|GetWorldLocation (Variables|Default|GetRadioMesh)) "0, 0, 0" 1.0 1.0 0.0 0 0))
  (Variables|Default|SetMusicPlayer _returnvalue)
  (EventDispatchers|BindEventtoOnAudioFinished (Variables|Default|GetMusicPlayer) (delegate Custom|Next%20Song)))

(event Custom|Next%20Song
  (bind _musicarray (Variables|Default|GetMusicArray))
  ;[0.15 0.15 0.15 0.5] Remove the current song from the array and place it back at the end
  (Variables|Default|SetTempVar (Utilities|Array|Get(acopy) _musicarray))
  (Utilities|Array|RemoveIndex _musicarray)
  (Utilities|Array|Add _musicarray (Variables|Default|GetTempVar))
  ;[0.15 0.15 0.15 0.5] Set new Sound
  (Audio|Components|Audio|SetSound (Variables|Default|GetMusicPlayer) (Utilities|Array|Get(acopy) (Variables|Default|GetMusicArray))))

(event Custom|Skip
  ;[0.15 0.15 0.15 0.5] Event for if the player manually skips a song
  (CallFunction|NextSong)
  (Development|PrintString "Next Song"))

(event EventBeginPlay
  (CallFunction|RadioStart))

(fn ConstructionScript)