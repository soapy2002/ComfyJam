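; Game manager that initialises the player and runs the day/night cycle.
; On BeginPlay it finds the "Sun"-tagged directional light and starts a slowed timeline at 4:00.
; Each timeline update pitches the sun by time of day, sends a formatted clock string to the player's HUD and sets a day flag, whose branch is still empty.
; GetHour exposes the current hour; FindHUD caches the HUD widget but is not called here.
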(event Custom|InitDayNightCycle
  (bind _daynightcycle (Variables|Default|GetDayNightCycle))
  (Components|Timeline|SetPlayRate _daynightcycle 0.1333)
  (Components|Timeline|SetPlaybackPosition _daynightcycle 4.0 false true)
  (bind _timeprog (Timeline|DayNightCycle Play)
    (:Update
      (bind _output_get (Variables|Default|SetTimeOfDay _timeprog))
      (Transformation|SetActorRotation (Variables|Default|GetTheSun) (Math|Rotator|MakeRotator 2.6e+02 (- (* _output_get 15.0) 2.7e+02) 2.7e+02))
      (bind _output_get_2 (Variables|Default|SetTime%20String (Utilities|Text|FormatText "{Hour}:{Minute}" (Math|Float|Truncate (Variables|Default|GetTimeOfDay)) (Math|Float|Truncate (* (- (Variables|Default|GetTimeOfDay) (Math|Float|Truncate (Variables|Default|GetTimeOfDay))) 6e+01)))))
      (Default|UpdateTime (Variables|/Game/Blueprints/BP_ComfyPlayer.BP_ComfyPlayer_C|GetPlayer%20Hud (Variables|Default|GetPlayer%20Ref)) _output_get_2)
      (bind _output_get_3 (Variables|Default|SetIsDay? (and (< (Variables|Default|GetTimeOfDay) 18.0) (> (Variables|Default|GetTimeOfDay) 6.0))))
      (if _output_get_3
        _))))

(event Custom|FindHUD
  (Utilities|FlowControl|Delay 0.2)
  (bind _foundwidgets (Widget|GetAllWidgetsOfClass "/Game/UserInterface/W_HUD.W_HUD_C" false))
  (Variables|Default|SetHUD (Utilities|Array|Get(acopy) _foundwidgets)))

(event EventBeginPlay
  (bind _outactors (Actor|GetAllActorsOfClasswithTag "/Script/Engine.DirectionalLight" "Sun"))
  (Variables|Default|SetTheSun (Utilities|Array|Get(acopy) _outactors))
  (bind _asbp_comfy_player (Utilities|Casting|CastToBP_ComfyPlayer (Game|GetPlayerCharacter 0)))
  (bind _output_get (Variables|Default|SetPlayer%20Ref _asbp_comfy_player))
  (Default|Initialise _output_get)
  (CallFunction|InitDayNightCycle))

(fn ConstructionScript)

(fn GetHour
  (return (Math|Float|Truncate (Variables|Default|GetTimeofDay))))